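; Actor component that holds a fixed-size inventory of Cores and handles player interaction with world objects.
; Each tick a forward sphere trace from the player pawn caches and prints the looked-at actor, which the interact input messages through its CoreData component.
; Slot helpers stack quantities by CoreID against Core data table limits.
; Adding is unfinished and unwired, removal is empty, and key 1 prints contents for debugging.
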(event Custom|Interaction
  (params (Target :type Actor%20Object%20Reference))
  (bind _returnvalue (Actor|GetComponentbyClass Target "/Game/Blueprint/Inventory_Equips/BP_Component_CoreData.BP_Component_CoreData_C"))
  (Utilities|IsValid _returnvalue
    (:Is%20Valid
      (Class|BPIInteraction|CanInteract(Message) _returnvalue))))

(event Input|EnhancedActionEvents|EnhancedInputActionIA_Interact
  (params (ActionValue :type Boolean) (ElapsedSeconds :type Float%20%28double-precision%29) (TriggeredSeconds :type Float%20%28double-precision%29) (InputAction :type Input%20Action%20Object%20Reference :default "/Game/Input/IA_Interact.IA_Interact"))
  (bind _lookatactor (Variables|Default|GetLookAtActor)
    (:then
      (CallFunction|Interaction _lookatactor))
    (:else)))

(event EventTick
  (params (DeltaSeconds :type Float%20%28single-precision%29))
  (CallFunction|InteractionTracing))

(event EventBeginPlay
  (Utilities|Array|Resize (Variables|Default|GetContent) (Variables|Default|GetCoreInventorySize)))

(event Input|KeyboardEvents|1
  (params (Key :type Key%20Structure :default "None"))
  (:Pressed
    (CallFunction|DEBUGPRINTCONTENT)))

(fn AddtoCoreInventory
  (params (CoreID :type Name) (Level :type Integer) (Quantity :type Integer) (Cost :type Integer))
  (bind (_index _has_empty_slot _item_id) (CallFunction|FindSlot CoreID))
  (while (< Quantity 4)
    (if _has_empty_slot
      (CallFunction|AddtoSlot _index 1)
      (if (== (+ (CallFunction|GetMaxQuantity _item_id) 1) 3)
        (return true 0))))
  (return false -1))

(fn RemovefromCoreInventory)

(fn InteractionTracing
  (bind _returnvalue (Game|Player|GetPlayerPawn 0))
  (bind _returnvalue_2 (Transformation|GetActorLocation _returnvalue))
  (bind (_outhit _returnvalue_3) (Collision|SphereTraceByChannel _returnvalue_2 (+ _returnvalue_2 (* (Transformation|GetActorForwardVector _returnvalue) (Variables|Default|GetInteractionRange))) 0.0 "TraceTypeQuery3" false (Utilities|Array|MakeArray (Components|GetOwner)) "None"))
  (if _returnvalue_3
    (if (!= (.HitActor (Collision|BreakHitResult _outhit)) (Variables|Default|GetLookAtActor))
      (bind _output_get (Variables|Default|SetLookAtActor (.HitActor (Collision|BreakHitResult _outhit))))
      (bind _messagetext (Class|BPIInteraction|Lookat(Message) _output_get))
      (Development|PrintString (Utilities|String|ToString(Text) _messagetext)))
    (else
      (Variables|Default|SetLookAtActor 0))))

(fn FindSlot
  (params (CoreID :type Name))
  (for (_array_element _array_index) (Variables|Default|GetContent)
    (if (== (.CoreID (Utilities|Struct|BreakFCoreSlotStruct _array_element)) CoreID)
      (if (< (.Quantity (Utilities|Struct|BreakFCoreSlotStruct _array_element)) (CallFunction|GetMaxQuantity CoreID))
        (return _array_index true CoreID))))
  (return -1 false "None"))

(fn AnyEmptySlot
  (for _array_element (Variables|Default|GetContent)
    (if (<= (.Quantity (Utilities|Struct|BreakFCoreSlotStruct _array_element)) 3)
      (return true (.CoreID (Utilities|Struct|BreakFCoreSlotStruct _array_element)))))
  (return false "None"))

(fn AddtoSlot
  (params (Index :type Integer) (Quantity :type Integer))
  (bind _content (Variables|Default|GetContent))
  (bind _output (Utilities|Array|Get(acopy) _content Index))
  (Utilities|Array|SetArrayElem (Variables|Default|GetContent) Index (Utilities|Struct|MakeFCoreSlotStruct (.coreid _output) (.cost _output) (.level _output) (+ (.quantity _output) Quantity))))

(fn DEBUGPRINTCONTENT
  (for (_array_element _array_index) (Variables|Default|GetContent)
    (Development|PrintString (Utilities|String|Append (Utilities|String|ToString(Integer) _array_index) "; " (Utilities|String|ToString(Name) (.CoreID (Utilities|Struct|BreakFCoreSlotStruct _array_element))) "== " (Utilities|String|ToString(Integer) (.Cost (Utilities|Struct|BreakFCoreSlotStruct _array_element))) "; " (Utilities|String|ToString(Integer) (.Level (Utilities|Struct|BreakFCoreSlotStruct _array_element))) "; " (Utilities|String|ToString(Integer) (.Quantity (Utilities|Struct|BreakFCoreSlotStruct _array_element)))))))

(fn GetMaxQuantity
  (params (ItemID :type Name))
  (bind _returnvalue (Utilities|GetDataTableRow "/Game/Blueprint/Inventory_Equips/Table_Core.Table_Core" ItemID)
    (:then
      (return (.Quantity (Utilities|Struct|BreakFCoreStruct _returnvalue))))
    (:RowNotFound
      (return -1))))

(fn NewFunction)

(fn Lookat
  (return ""))