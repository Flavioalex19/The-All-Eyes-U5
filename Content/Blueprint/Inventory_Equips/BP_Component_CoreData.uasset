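; Actor component for a core pickup, handling interaction with the item in the world.
; On CanInteract it prints a debug string, re-adds the first element of the passed core array to that array, then destroys its owner.
; An unconnected branch would add the core's ID, quantity and cost to the player's CoreInventory component and destroy the owner on success.
; LookAt returns an empty string.
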(event EventCanInteract
  (params (ArrayCore :type Array%20of%20F%20Core%20Slot%20Struct%20Structures) (index :type Integer))
  (Development|PrintString "received")
  (bind _array_element (Utilities|Array|ForEachLoopwithBreak ArrayCore :!label _label)
    (:LoopBody
      (if true
        (Utilities|Array|Add ArrayCore _array_element)
        (Actor|DestroyActor (Components|GetOwner))
        (goto _label Break)))))

(fn Lookat
  (return ""))