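; BP_Component_CoreData is an unfinished component that describes a Core item by ID, cost and quantity, apparently for pickup into the player's core inventory.
; Its CanInteract event only loops over the passed Core array, appends each element back onto it and prints "Added".
; Work-in-progress logic to fill BPComponent_CoreInventory on the player pawn, print its contents and destroy the owner is disconnected and never runs.
; LookAt returns an empty string.
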(event EventCanInteract
  (params (ArrayCore :type Array%20of%20F%20Core%20Slot%20Struct%20Structures) (index :type Integer))
  (Utilities|Array|ForEachLoopwithBreak ArrayCore
    (:LoopBody
      (if true
        (Utilities|Array|Add :TargetArray ArrayCore)
        (Development|PrintString "Added")))))

(fn Lookat
  (return ""))