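; BP_Core is a pickup actor for a Core item that announces itself to the player through a box overlap.
; Entering or leaving the Box sets IsInteracted and passes it with CoreData to player pawn 0 via InteractedMessage, without checking which actor overlapped.
; DestroyItem removes the actor.
; LookAt is empty, and its "Pick Up {item}" prompt formatting is disconnected.
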(event OnComponentBeginOverlap(Box)
  (params (OverlappedComponent :type Primitive%20Component%20Object%20Reference) (OtherActor :type Actor%20Object%20Reference) (OtherComp :type Primitive%20Component%20Object%20Reference) (OtherBodyIndex :type Integer) (bFromSweep :type Boolean) (SweepResult :type Hit%20Result%20Structure%20%28by%20ref%29))
  (bind _output_get (Variables|Default|SetIs%20interacted true))
  (Class|BPICoreInteraction|Interacted(Message) (Game|Player|GetPlayerPawn 0) _output_get (Variables|Default|GetCore%20Data)))

(event OnComponentEndOverlap(Box)
  (params (OverlappedComponent :type Primitive%20Component%20Object%20Reference) (OtherActor :type Actor%20Object%20Reference) (OtherComp :type Primitive%20Component%20Object%20Reference) (OtherBodyIndex :type Integer))
  (bind _output_get (Variables|Default|SetIs%20interacted false))
  (Class|BPICoreInteraction|Interacted(Message) (Game|Player|GetPlayerPawn 0) _output_get (Variables|Default|GetCore%20Data)))

(event EventDestroyItem
  (Actor|DestroyActor))

(fn ConstructionScript)

(fn Lookat)