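; BP_Dialogue_Manager controls the on-screen dialogue box shown during conversations.
; On BeginPlay it creates a WB_DialogueBox widget and adds it to the viewport.
; Start and end conversation events set a flag that Tick polls every frame to show or hide the box.
; A separate update event writes the text passed by the caller into the box.
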(event EventDialogueTextUpdate
  (params (DT_Row :type Text))
  ;[1 1 1] Updates the Dialogue Text on the Dialogue Box
  (Rendering|Components|TextRender|SetText (Variables|/Game/Widgets/WB_DialogueBox.WB_DialogueBox_C|GetDialogueText (stale EventBeginPlay _returnvalue)) DT_Row))

(event EventBeginPlay
  ;[1 1 1] Updates the Dialogue Text on the Dialogue Box
  (bind _returnvalue (UserInterface|CreateWidget "/Game/Widgets/WB_DialogueBox.WB_DialogueBox_C"))
  (UserInterface|Viewport|AddtoViewport _returnvalue 0))

(event EventDialogueEndConversation
  (params (Is%20On :type Boolean))
  ;[1 1 1] End Conversation to set dialogue panel to hidden
  (Variables|Default|SetIs%20Dialogue%20Panel%20on false))

(event EventTick
  (params (DeltaSeconds :type Float%20%28single-precision%29))
  ;[1 1 1] Updates the Dialogue Text on the Dialogue Box
  (if (Variables|Default|GetIs%20Dialogue%20Panel%20on)
    (Variables|/Script/UMG.Widget|SetVisibility (stale EventBeginPlay _returnvalue) "Visible")
    (else
      (Variables|/Script/UMG.Widget|SetVisibility (stale EventBeginPlay _returnvalue) "Hidden"))))

(event EventDialogueStartConversation
  (params (Is%20On :type Boolean))
  ;[1 1 1] Start Conversation to set dialogue panel on
  (Variables|Default|SetIs%20Dialogue%20Panel%20on true))

(fn ConstructionScript)