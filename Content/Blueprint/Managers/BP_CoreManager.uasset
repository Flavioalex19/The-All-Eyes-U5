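; BP_CoreManager is an early-stage manager for assigning skill core types to active skill core slots.
; AddCore writes the type to the given slot, prints it, then calls CastCoreMessage on the stored slot A rather than that slot.
; Tick prints slot A's type as debug output, though no executed node here sets slot A.
; CastCore is a stub returning a fixed enum value.
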(event EventAddCore
  (params (Active%20Skill%20Core%20Slot :type BP%20Skill%20Core%20Object%20Reference) (Skill%20Core%20Type :type Skills_Cores%20Enum :default "NewEnumerator0"))
  (bind _output_get (Variables|/Game/Blueprint/Skills/BP_SkillCore.BP_SkillCore_C|SetSkill%20Core%20Type Active%20Skill%20Core%20Slot Skill%20Core%20Type))
  (Development|PrintString (Utilities|String|EnumtoString _output_get))
  (Class|BPICoreManager|CastCore(Message) (Variables|Default|GetActive%20Skill%20Core%20Slot%20A)))

(event EventTick
  (params (DeltaSeconds :type Float%20%28single-precision%29))
  (Development|PrintString (Utilities|String|EnumtoString (Variables|/Game/Blueprint/Skills/BP_SkillCore.BP_SkillCore_C|GetSkill%20Core%20Type (Variables|Default|GetActive%20Skill%20Core%20Slot%20A)))))

(fn ConstructionScript)

(fn CastCore
  (return "NewEnumerator0"))