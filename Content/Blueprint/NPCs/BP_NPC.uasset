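; BP_NPC is a non-player character that steps through its own array of dialogue lines each time its Talk event fires.
; After a short delay, it finds BP_Dialogue_Manager in the level, signals conversation start, and sends the current line and array length to the first manager implementing BPI_Dialogue.
; Once the lines run out, it resets the index, clears IsTalking and tells the manager to end the conversation.
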(event EventTalk
  ;[1 1 1] Talk Event Trigger
  (Math|Integer|IncrementInt (Variables|Default|GetTalk%20Index)
    (:%20%20
      (Utilities|FlowControl|Delay 0.2)
      (if (< (Variables|Default|GetTalk%20Index) (Utilities|Array|Length (Variables|Default|GetDialogue%20Array)))
        (Variables|Default|SetIs%20talking true)
        (bind _returnvalue (Actor|GetActorOfClass "/Game/Blueprint/Managers/BP_Dialogue_Manager.BP_Dialogue_Manager_C"))
        (Class|BPIDialogue|DialogueStartConversation(Message) _returnvalue false)
        (bind _outactors (Actor|GetAllActorsOfClass "/Game/Blueprint/Managers/BP_Dialogue_Manager.BP_Dialogue_Manager_C"))
        (bind _array_element (Utilities|Array|ForEachLoopwithBreak _outactors :!label _label)
          (:LoopBody
            (if (Utilities|DoesObjectImplementInterface _array_element "/Game/Blueprint/Interface/BPI_Dialogue.BPI_Dialogue_C")
              (Class|BPIDialogue|DialogueTextUpdate(Message) _array_element (Utilities|Array|Get(acopy) (Variables|Default|GetDialogue%20Array) (Variables|Default|GetTalk%20Index)) (Utilities|Array|Length (Variables|Default|GetDialogue%20Array)))
              (goto _label Break))))
        (else
          (Variables|Default|SetTalk%20Index -1)
          (bind _output_get (Variables|Default|SetIs%20talking false))
          (bind _returnvalue_2 (Actor|GetActorOfClass "/Game/Blueprint/Managers/BP_Dialogue_Manager.BP_Dialogue_Manager_C"))
          (Default|DialogueEndConversation _returnvalue_2 _output_get))))))

(fn ConstructionScript)