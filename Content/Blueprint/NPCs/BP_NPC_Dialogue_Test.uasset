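; Test NPC Blueprint for a dialogue system, currently inert: Talk is empty and LookAt returns an empty string.
; Disconnected logic would step DialogueIndex through the Dialogue array, set IsTalking, and message BP_Dialogue_Manager to start or end the conversation.
; It would also send text updates via BPI_Dialogue using DT_DialogueSystem with a blank row, leaving the current array line unused.
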(event EventTalk)

(fn ConstructionScript)

(fn Lookat
  (return ""))