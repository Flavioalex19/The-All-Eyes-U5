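; BP_SkillCore handles activation of the player's skill core, dispatching by SkillCoreType to wind or fire abilities.
; On BeginPlay it caches the player character and its placeholder animation Blueprint instance.
; ActivateGeneralCore switches on the core type, calling the matching wind or fire activation message with a debug print.
; The remaining case reports that no core is activated and plays a collapse sound.
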(event EventBeginPlay
  (References|ThirdPersonCharacterRef)
  (References|TPCABPRef))

(event EventActivateGeneralCore
  (switch Utilities|FlowControl|Switch|SwitchonSkills_Cores (Variables|Default|GetSkill%20Core%20Type)
    (:NewEnumerator0
      (Development|PrintString "Not activated")
      (Audio|PlaySound2D "/Game/StarterContent/Audio/Collapse_Cue.Collapse_Cue" 1.0 1.0 0.0 0 0))
    (:NewEnumerator1
      (Development|PrintString "active wind  core")
      (Class|BPICoreManager|ActivateWindCore(Message) self))
    (:NewEnumerator2
      (Development|PrintString "active fire core")
      (Class|BPICoreManager|ActivateFireCore(Message) self))))

(fn ConstructionScript)

(fn ThirdPersonCharacterRef
  (Variables|References|SetThird%20Person%20Character%20Reference (Game|GetPlayerCharacter 0)))

(fn TPCABPRef
  (bind _asab_placeholder_chracter (Utilities|Casting|CastToAB_Placeholder_Chracter (Components|SkeletalMesh|GetAnimInstance (Variables|/Script/Engine.Character|GetMesh (Game|GetPlayerCharacter 0)))))
  (Variables|References|SetABP%20Third%20Person%20Character%20Reference _asab_placeholder_chracter))