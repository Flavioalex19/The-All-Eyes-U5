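; BP_Altar is an interactable altar that toggles a widget, held as WBCoresObjectRef, on and off the screen.
; BeginPlay creates the widget for the first player controller from WidgetClass.
; Each AltarInteraction call alternates through a FlipFlop between showing and removing it, updating UIIsOn, the mouse cursor and InteractedItem on the BP_KesterV_01 player character.
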(event EventBeginPlay
  (bind _returnvalue (UserInterface|CreateWidget (Variables|Default|GetWidget_Class) (Game|GetPlayerController 0)))
  (Variables|Default|SetWB_Cores%20Object%20Ref _returnvalue))

(event EventTick
  (params (DeltaSeconds :type Float%20%28single-precision%29))
  (|CallParentFunction DeltaSeconds) ; This node is disabled and will not be called.\nDrag off pins to build functionality.
)

(event EventAltarInteraction
  (bind _wb_cores_object_ref (Variables|Default|GetWB_Cores%20Object%20Ref))
  (Utilities|IsValid _wb_cores_object_ref
    (:Is%20Valid
      (Utilities|FlowControl|FlipFlop
        (:A
          (UserInterface|Viewport|AddtoViewport _wb_cores_object_ref 0)
          (Variables|Default|SetUI%20is%20On true)
          (Variables|/Script/Engine.PlayerController|SetbShowMouseCursor (Game|GetPlayerController 0) true)
          (bind _asbp_kester_v_01 (Utilities|Casting|CastToBP_KesterV_01 (Game|GetPlayerCharacter 0)))
          (Variables|/Game/Blueprint/Character/BP_KesterV_01.BP_KesterV_01_C|SetInteracted_Item _asbp_kester_v_01 true))
        (:B
          (Widget|RemovefromParent _wb_cores_object_ref)
          (Variables|Default|SetUI%20is%20On false)
          (Variables|/Script/Engine.PlayerController|SetbShowMouseCursor (Game|GetPlayerController 0) false)
          (bind _asbp_kester_v_01_2 (Utilities|Casting|CastToBP_KesterV_01 (Game|GetPlayerCharacter 0)))
          (Variables|/Game/Blueprint/Character/BP_KesterV_01.BP_KesterV_01_C|SetInteracted_Item _asbp_kester_v_01_2 false))))))

(fn ConstructionScript
  (|CallParentFunction))