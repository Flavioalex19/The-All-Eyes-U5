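; BP_NPC3 is an interactable NPC that advances through dialogue rows from DT_Dialogue2 on Talk.
; Each Talk increments an index, signals conversation start and sends the row's content to BP_Dialogue_Manager actors implementing BPI_Dialogue.
; The in-loop end check compares the index against DT_DialogueSystem's row count, a different table from the one read.
; Running past DT_Dialogue2's rows resets the index and signals conversation end.
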(event EventTalk
  (bind _outrownames (DataTable|GetDataTableRowNames "/Game/Blueprint/NPCs/Dialogue_SystemNPC/DT_Dialogue2.DT_Dialogue2"))
  (bind _result (Math|Integer|IncrementInt (Variables|Default|GetIndex))
    (:%20%20
      (if (< _result (Utilities|Array|Length _outrownames))
        (bind _output_get (Variables|Default|SetIs%20talking true))
        (bind _returnvalue (Utilities|GetDataTableRow "/Game/Blueprint/NPCs/Dialogue_SystemNPC/DT_Dialogue2.DT_Dialogue2" (Utilities|Array|Get(acopy) _outrownames (Variables|Default|GetIndex)))
          (:then
            (bind _returnvalue_2 (Actor|GetActorOfClass "/Game/Blueprint/Managers/BP_Dialogue_Manager.BP_Dialogue_Manager_C"))
            (Class|BPIDialogue|DialogueStartConversation(Message) _returnvalue_2 _output_get)
            (bind _outactors (Actor|GetAllActorsOfClass "/Game/Blueprint/Managers/BP_Dialogue_Manager.BP_Dialogue_Manager_C"))
            (bind _array_element (Utilities|Array|ForEachLoopwithBreak _outactors :!label _label)
              (:LoopBody
                (if (Utilities|DoesObjectImplementInterface _array_element "/Game/Blueprint/Interface/BPI_Dialogue.BPI_Dialogue_C")
                  (Class|BPIDialogue|DialogueTextUpdate(Message) _array_element (.dialoguecontent _returnvalue))
                  (bind _outrownames_2 (DataTable|GetDataTableRowNames "/Game/Blueprint/NPCs/Dialogue_SystemNPC/DT_DialogueSystem.DT_DialogueSystem"))
                  (if (>= (Variables|Default|GetIndex) (Utilities|Array|Length _outrownames_2))
                    (bind _output_get_2 (Variables|Default|SetIs%20Talking false))
                    (Class|BPIDialogue|DialogueEndConversation(Message) _array_element _output_get_2)
                    (goto _label Break)))))))
        (else
          (bind _output_get_3 (Variables|Default|SetIs%20talking false))
          (Variables|Default|SetIndex -1)
          (bind _returnvalue_3 (Actor|GetActorOfClass "/Game/Blueprint/Managers/BP_Dialogue_Manager.BP_Dialogue_Manager_C"))
          (Class|BPIDialogue|DialogueEndConversation(Message) _returnvalue_3 _output_get_3))))))

(fn ConstructionScript
  (|CallParentFunction))