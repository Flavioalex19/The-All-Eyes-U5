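; Runtime updater for a dynamic smear effect, feeding per-bone smear vectors to materials through a render target.
; Samples points along tracked bones, interpolates trailing smear ends and gradually rotates them opposite the movement.
; Draws positions, vectors and settings as pixels, one column per point, with negating bones adding positions too.
; Shares history through the master component to skip already-updated bones, and switches catch-up speed while fading out before disabling.
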(event Custom|Update
  (params (RenderTargetCanvas :type Canvas%20Object%20Reference))
  (bind _smeardata (Variables|Default|GetSmearData))
  (bind (_trackedbones _negatingbones _density _pullangle _midpoint _spikevariation _maxdistancefrombone _catchupspeed _catchupspeedwhenoff) (Utilities|Struct|BreakST_BoneSmearData _smeardata))
  (CallFunction|UpdateBoneSmearVectors RenderTargetCanvas (Math|Float|SelectFloat _catchupspeedwhenoff _catchupspeed (Variables|Default|GetFadingOut))))

(event Custom|Fade%20off
  (bind _smeardata (Variables|Default|GetSmearData))
  (bind (_trackedbones _negatingbones _density _pullangle _midpoint _spikevariation _maxdistancefrombone _catchupspeed _catchupspeedwhenoff) (Utilities|Struct|BreakST_BoneSmearData _smeardata))
  (Variables|Default|SetFadingOut true)
  (Utilities|FlowControl|Delay (Default|GetSmearTimeLefttoTarget (Variables|Default|GetMaster%20Smear%20Component) _trackedbones _catchupspeedwhenoff))
  (Variables|Default|SetEnabled false))

(event Custom|Turn%20off
  (Variables|Default|SetEnabled false))

(fn Initialize
  (params (MasterSmearComponent :type AC%20Dynamic%20Smears%20Object%20Reference) (Owning%20ANS :type Anim%20Notify%20State%20Object%20Reference%20%28by%20ref%29) (MaterialInstances :type Array%20of%20Material%20Instance%20Dynamic%20Object%20References) (SkinnedMesh :type Skinned%20Mesh%20Component%20Object%20Reference) (SmearRenderTarget :type Texture%20Render%20Target%202D%20Object%20Reference) (SmearData :type ST%20Bone%20Smear%20Data%20Structure) (PointsPerBone :type Map%20of%20Names%20to%20Integers) (BoneLengths :type Map%20of%20Names%20to%20Reals) (BoneChildName :type Map%20of%20Names%20to%20Names))
  (Variables|Default|SetMaster%20Smear%20Component MasterSmearComponent)
  (Variables|Default|SetOwning%20ANS Owning%20ANS)
  (Variables|Default|SetMaterialInstances MaterialInstances)
  (Variables|Default|SetSkinnedMesh SkinnedMesh)
  (Variables|Default|SetSmearRenderTarget SmearRenderTarget)
  (Variables|Default|SetSmearData SmearData)
  (Variables|Default|SetPointsPerBone PointsPerBone)
  (Variables|Default|SetBoneLengths BoneLengths)
  (Variables|Default|SetBoneChildName BoneChildName)
  (CallFunction|SaveTrackedBoneData)
  (return self))

(fn SaveDatatoRenderTarget
  (params (Canvas :type Canvas%20Object%20Reference) (Pixel%20X :type Integer) (Pixel%20Y :type Integer) (Data :type Linear%20Color%20Structure))
  (Canvas|DrawTexture :self Canvas :ScreenPosition (Math|Vector2D|MakeVector2D (Math|Conversions|ToFloat(Integer) Pixel%20X) (Math|Conversions|ToFloat(Integer) Pixel%20Y)) :ScreenSize "(X=1.000000,Y=1.000000)" :CoordinateSize "(X=1.000000,Y=1.000000)" :RenderColor Data :BlendMode "BLEND_Opaque" :PivotPoint "(X=0.000000,Y=0.000000)"))

(fn GetBonePoints
  (params (BoneName :type Name))
  (bind _skinnedmesh (Variables|Default|GetSkinnedMesh))
  (bind _bonechildname (Variables|Default|GetBoneChildName))
  (bind _bonelengths (Variables|Default|GetBoneLengths))
  (bind _pointsperbone (Variables|Default|GetPointsPerBone))
  (bind (_value _returnvalue) (Utilities|Map|Find _bonelengths BoneName))
  (bind (_value_2 _returnvalue_2) (Utilities|Map|Find _pointsperbone BoneName))
  (bind _returnvalue_3 (Transformation|GetBoneTransform _skinnedmesh BoneName "RTS_World"))
  (bind (_value_3 _returnvalue_4) (Utilities|Map|Find _bonechildname BoneName))
  (LocalVariables|SetNumberOfPoints (Math|Integer|SelectInt _value_2 (Variables|Default|GetPointsPerBoneDefault) _returnvalue_2))
  (LocalVariables|SetPointDistance (/ (Math|Float|SelectFloat _value 0.0 _returnvalue) (+ (LocalVariables|GetNumberOfPoints) 1)))
  (for _index (range 1 (LocalVariables|GetNumberOfPoints))
    (Utilities|Array|Add (LocalVariables|GetPointsToReturn) (+ (.location _returnvalue_3) (* (CallFunction|DirectionNorm (.location _returnvalue_3) (.location (Transformation|GetBoneTransform (Variables|Default|GetSkinnedMesh) (select _returnvalue_4 _value_3 BoneName) "RTS_World"))) (* (LocalVariables|GetPointDistance) _index)))))
  (return (LocalVariables|GetPointsToReturn)))

(fn UpdateBoneSmearVectors
  (params (RenderTargetCanvas :type Canvas%20Object%20Reference) (SmearCatchupSpeedToUse :type Float%20%28single-precision%29))
  (bind _smeardata (Variables|Default|GetSmearData))
  (bind _smeardata_2 (Variables|Default|GetSmearData))
  (bind (_trackedbones _negatingbones) (Utilities|Struct|BreakST_BoneSmearData _smeardata))
  (bind (_trackedbones_2 _negatingbones_2 _density _pullangle _midpoint _spikevariation _maxdistancefrombone _catchupspeed _catchupspeedwhenoff _bonetosmearmaxangle _anglecatchupspeed) (Utilities|Struct|BreakST_BoneSmearData _smeardata_2))
  (Utilities|FlowControl|Sequence
    (:then_0
      (for _array_element _trackedbones
        (LocalVariables|SetCurrentBoneName _array_element)
        (if (or (not (.ReturnValue (Utilities|Map|Find (Variables|/Game/DynamicSmears/Blueprints/Components/AC_DynamicSmears.AC_DynamicSmears_C|GetSharedBoneTrackingData (Variables|Default|GetMaster%20Smear%20Component)) (LocalVariables|GetCurrentBoneName)))) (not (.Updated (Utilities|Struct|BreakST_BoneTrackingData (.Value (Utilities|Map|Find (Variables|/Game/DynamicSmears/Blueprints/Components/AC_DynamicSmears.AC_DynamicSmears_C|GetSharedBoneTrackingData (Variables|Default|GetMaster%20Smear%20Component)) (LocalVariables|GetCurrentBoneName)))))))
          (Utilities|Array|Clear (LocalVariables|GetUpdatedSmearEnds))
          (Utilities|Array|Clear (LocalVariables|GetUpdatedPreviousLocations))
          (bind _points (CallFunction|GetBonePoints (LocalVariables|GetCurrentBoneName)))
          (for (_array_element_2 _array_index) _points
            (CallFunction|SendSettingstoRenderTarget RenderTargetCanvas)
            (LocalVariables|SetCurrentBonePoint _array_element_2)
            (Utilities|FlowControl|Sequence
              (:then_0
                ;[1 1 1] Send bone position to material by drawing it on the render texture used in the material
                (CallFunction|SaveDatatoRenderTarget RenderTargetCanvas (Utilities|RTColIndex) (Variables|Default|GetROW_CURRENT_BONE_POSITION) (Math|Conversions|ToLinearColor(Vector) (LocalVariables|GetCurrentBonePoint)))
                ;;[1 0.5357 0.2708] Toggle the boolean to display debug info
                (if false
                  (Rendering|Debug|DrawDebugSphere (LocalVariables|GetCurrentBonePoint) 7.0 6 "(R=1.000000,G=0.049112,B=0.438972,A=1.000000)" 0.0 1.0)
                  (Rendering|Debug|DrawDebugString (LocalVariables|GetCurrentBonePoint) (Utilities|String|Append (Utilities|String|ToString(Name) (LocalVariables|GetCurrentBoneName)) " | " (Utilities|String|ToString(Vector) (LocalVariables|GetCurrentBonePoint))) 0 (Math|Color|SelectColor "(R=1.000000,G=0.091212,B=0.000000,A=1.000000)" "(R=1.000000,G=1.000000,B=1.000000,A=1.000000)" (Variables|Default|GetFadingOut)))))
              (:then_1
                ;[1 1 1] Process smear target and movement direction
                (if (.ReturnValue (Utilities|Map|Find (Variables|/Game/DynamicSmears/Blueprints/Components/AC_DynamicSmears.AC_DynamicSmears_C|GetSharedBoneTrackingData (Variables|Default|GetMaster%20Smear%20Component)) (LocalVariables|GetCurrentBoneName)))
                  (LocalVariables|SetSmearEndLocationUsed (Math|Interpolation|VInterpTo (Utilities|Array|Get(acopy) (.SmearEndLocations (Utilities|Struct|BreakST_BoneTrackingData (.Value (Utilities|Map|Find (Variables|/Game/DynamicSmears/Blueprints/Components/AC_DynamicSmears.AC_DynamicSmears_C|GetSharedBoneTrackingData (Variables|Default|GetMaster%20Smear%20Component)) (LocalVariables|GetCurrentBoneName))))) _array_index) (LocalVariables|GetCurrentBonePoint) (Utilities|Time|GetWorldDeltaSeconds) SmearCatchupSpeedToUse))
                  (LocalVariables|SetMovementDirection (- (LocalVariables|GetCurrentBonePoint) (Utilities|Array|Get(acopy) (.PreviousLocations (Utilities|Struct|BreakST_BoneTrackingData (.Value (Utilities|Map|Find (Variables|/Game/DynamicSmears/Blueprints/Components/AC_DynamicSmears.AC_DynamicSmears_C|GetSharedBoneTrackingData (Variables|Default|GetMaster%20Smear%20Component)) (LocalVariables|GetCurrentBoneName))))) _array_index)))
                  (if true
                    _)
                  (else
                    (LocalVariables|SetSmearEndLocationUsed (LocalVariables|GetCurrentBonePoint)))))
              (:then_2
                (LocalVariables|SetSmearDirection (- (LocalVariables|GetSmearEndLocationUsed) (LocalVariables|GetCurrentBonePoint))))
              (:then_3
                ;[1 0.5357 0.2708] Toggle the boolean to display debug info
                (if false
                  (Rendering|Debug|DrawDebugArrow (LocalVariables|GetCurrentBonePoint) (+ (LocalVariables|GetCurrentBonePoint) (CallFunction|ResizeVector (* (LocalVariables|GetMovementDirection) -1.0) 1e+02)) 1.0 "(R=0.000000,G=0.428552,B=1.000000,A=1.000000)" 0.0 1.0)
                  (Rendering|Debug|DrawDebugArrow (LocalVariables|GetCurrentBonePoint) (+ (LocalVariables|GetCurrentBonePoint) (CallFunction|ResizeVector (LocalVariables|GetSmearDirection) 1e+02)) 1.0 "(R=1.000000,G=0.477530,B=0.000000,A=1.000000)" 0.0 1.0)))
              (:then_4
                ;[1 1 1] Ensure than the smear is following the movement direction to some extend
                (if (and (> (Math|Vector|VectorLength (LocalVariables|GetMovementDirection)) 0.01) (> (CallFunction|AngleBetweenVectors (* (LocalVariables|GetMovementDirection) -1.0) (LocalVariables|GetSmearDirection)) _bonetosmearmaxangle))
                  (LocalVariables|SetSmearEndLocationUsed (+ (LocalVariables|GetCurrentBonePoint) (Math|Vector|SelectVector (Math|Vector|RotateVectorAroundAxis (LocalVariables|GetSmearDirection) (Math|Float|Min(Float) (CallFunction|AngleBetweenVectors (* (LocalVariables|GetMovementDirection) -1.0) (LocalVariables|GetSmearDirection)) (* _anglecatchupspeed (Utilities|Time|GetWorldDeltaSeconds))) (Math|Vector|CrossProduct (CallFunction|Norm (LocalVariables|GetMovementDirection)) (CallFunction|Norm (LocalVariables|GetSmearDirection)))) (Math|Vector|RotateVectorAroundAxis (LocalVariables|GetSmearDirection) (* (Math|Float|Min(Float) (CallFunction|AngleBetweenVectors (* (LocalVariables|GetMovementDirection) -1.0) (LocalVariables|GetSmearDirection)) (* _anglecatchupspeed (Utilities|Time|GetWorldDeltaSeconds))) -1.0) (Math|Vector|CrossProduct (CallFunction|Norm (LocalVariables|GetMovementDirection)) (CallFunction|Norm (LocalVariables|GetSmearDirection)))) (<= (CallFunction|AngleBetweenVectors (* (LocalVariables|GetMovementDirection) -1.0) (Math|Vector|RotateVectorAroundAxis (LocalVariables|GetSmearDirection) (Math|Float|Min(Float) (CallFunction|AngleBetweenVectors (* (LocalVariables|GetMovementDirection) -1.0) (LocalVariables|GetSmearDirection)) (* _anglecatchupspeed (Utilities|Time|GetWorldDeltaSeconds))) (Math|Vector|CrossProduct (CallFunction|Norm (LocalVariables|GetMovementDirection)) (CallFunction|Norm (LocalVariables|GetSmearDirection))))) (CallFunction|AngleBetweenVectors (* (LocalVariables|GetMovementDirection) -1.0) (LocalVariables|GetSmearDirection))))))))
              (:then_5
                ;[1 1 1] Send smear direction to material
                (CallFunction|SaveDatatoRenderTarget RenderTargetCanvas (Utilities|RTColIndex) (Variables|Default|GetROW_SMEAR_DIRECTION) (Math|Conversions|ToLinearColor(Vector) (- (LocalVariables|GetSmearEndLocationUsed) (LocalVariables|GetCurrentBonePoint))))
                ;[1 0.5357 0.2708] Toggle the boolean to display debug info
                (if false
                  (Rendering|Debug|DrawDebugSphere (LocalVariables|GetSmearEndLocationUsed) 7.0 6 "(R=1.000000,G=0.771949,B=0.000000,A=1.000000)" 0.0 1.0)
                  (Rendering|Debug|DrawDebugString (LocalVariables|GetSmearEndLocationUsed) (Utilities|String|Append (Utilities|String|ToString(Name) (LocalVariables|GetCurrentBoneName)) "Smear target  | " (Utilities|String|ToString(Vector) (LocalVariables|GetSmearEndLocationUsed)) " | Speed: " (Utilities|String|ToString(Float) SmearCatchupSpeedToUse)) 0 (Math|Color|SelectColor "(R=1.000000,G=0.091212,B=0.000000,A=1.000000)" "(R=1.000000,G=1.000000,B=1.000000,A=1.000000)" (Variables|Default|GetFadingOut)))))
              (:then_6
                ;[1 1 1] Record movement for next update
                (Utilities|Array|Add (LocalVariables|GetUpdatedSmearEnds) (LocalVariables|GetSmearEndLocationUsed))
                (Utilities|Array|Add (LocalVariables|GetUpdatedPreviousLocations) (LocalVariables|GetCurrentBonePoint)))
              (:then_7
                ;[1 1 1] End sequence
                (Math|Integer|IncrementInt (Variables|/Game/DynamicSmears/Blueprints/Components/AC_DynamicSmears.AC_DynamicSmears_C|GetRTColIndex (Variables|Default|GetMaster%20Smear%20Component))))))
          (CallFunction|SavetoShared (LocalVariables|GetCurrentBoneName) (LocalVariables|GetUpdatedSmearEnds) (LocalVariables|GetUpdatedPreviousLocations) (.CatchupSpeedWhenOff (Utilities|Struct|BreakST_BoneSmearData (Variables|Default|GetSmearData)))))))
    (:then_1
      (for _array_element_3 _negatingbones
        (bind _points_2 (CallFunction|GetBonePoints _array_element_3))
        (for _array_element_4 _points_2
          (CallFunction|SaveDatatoRenderTarget RenderTargetCanvas (Utilities|RTColIndex) (Variables|Default|GetROW_CURRENT_BONE_POSITION) (Math|Conversions|ToLinearColor(Vector) _array_element_4))
          (CallFunction|SaveDatatoRenderTarget RenderTargetCanvas (Utilities|RTColIndex) (Variables|Default|GetROW_SMEAR_DIRECTION))
          (Math|Integer|IncrementInt (Variables|/Game/DynamicSmears/Blueprints/Components/AC_DynamicSmears.AC_DynamicSmears_C|GetRTColIndex (Variables|Default|GetMaster%20Smear%20Component))))))))

(fn SaveTrackedBoneData
  (bind _smeardata (Variables|Default|GetSmearData))
  (bind (_trackedbones _negatingbones) (Utilities|Struct|BreakST_BoneSmearData _smeardata))
  (LocalVariables|SetSocketAndBoneNames (Transformation|GetAllSocketNames (Variables|Default|GetSkinnedMesh)))
  (Utilities|Array|AppendArray (LocalVariables|GetBonesToRecord) _trackedbones)
  (Utilities|Array|AppendArray (LocalVariables|GetBonesToRecord) _negatingbones)
  (for _array_element (LocalVariables|GetBonesToRecord)
    (LocalVariables|SetCurrentBoneIndex (Class|SkinnedMeshComponent|GetBoneIndex (Variables|Default|GetSkinnedMesh) _array_element))
    (LocalVariables|SetCurrentBoneTransform (Transformation|GetBoneTransform (Variables|Default|GetSkinnedMesh) _array_element "RTS_World"))
    (for _array_element_2 (LocalVariables|GetSocketAndBoneNames)
      (if (== (Class|SkinnedMeshComponent|GetBoneIndex (Variables|Default|GetSkinnedMesh) _array_element_2) (+ (LocalVariables|GetCurrentBoneIndex) 1))
        ;[1 1 1] Record length if there is no record yet, or if the found length is longer than the recorded one
        (if (.ReturnValue (Utilities|Map|Find (Variables|Default|GetBoneLengths) _array_element))
          (if (> (Math|Vector|VectorLength (- (.location (Transformation|GetBoneTransform (Variables|Default|GetSkinnedMesh) _array_element_2 "RTS_World")) (.location (LocalVariables|GetCurrentBoneTransform)))) (.Value (Utilities|Map|Find (Variables|Default|GetBoneLengths) _array_element)))
            (Utilities|Map|Add (Variables|Default|GetBoneLengths) _array_element (Math|Vector|VectorLength (- (.location (Transformation|GetBoneTransform (Variables|Default|GetSkinnedMesh) _array_element_2 "RTS_World")) (.location (LocalVariables|GetCurrentBoneTransform)))) :!label _label)
            (Utilities|Map|Add (Variables|Default|GetBoneChildName) _array_element _array_element_2))
          (else
            (goto _label)))))
    ;[1 1 1] If the bone has no child, set is length to a default of 0
    (if (not (.ReturnValue (Utilities|Map|Find (Variables|Default|GetBoneLengths) _array_element)))
      (Utilities|Map|Add (Variables|Default|GetBoneLengths) _array_element 0.0))))

(fn SendSettingstoRenderTarget
  (params (Canvas :type Canvas%20Object%20Reference))
  (bind _smeardata (Variables|Default|GetSmearData))
  (bind (_trackedbones _negatingbones _density _pullangle _midpoint _spikevariation _maxdistancefrombone) (Utilities|Struct|BreakST_BoneSmearData _smeardata))
  (CallFunction|SaveDatatoRenderTarget Canvas (Utilities|RTColIndex) (Variables|Default|GetROW_DATA_DENS_PULL_MID_SPIKE) (Utilities|Struct|MakeLinearColor _density _pullangle _midpoint _spikevariation))
  (CallFunction|SaveDatatoRenderTarget Canvas (Utilities|RTColIndex) (Variables|Default|GetROW_DATA_DIST) (Utilities|Struct|MakeLinearColor _maxdistancefrombone 0.0 0.0 0.0)))

(fn SavetoShared
  (params (Bone%20name :type Name%20%28by%20ref%29) (UpdatedSmearEndLocations :type Array%20of%20Vectors) (UpdatedPreviousLocations :type Array%20of%20Vectors) (CatchupSpeed :type Float%20%28double-precision%29))
  (Utilities|Map|Add (Variables|/Game/DynamicSmears/Blueprints/Components/AC_DynamicSmears.AC_DynamicSmears_C|GetSharedBoneTrackingData (Variables|Default|GetMaster%20Smear%20Component)) Bone%20name (Utilities|Struct|MakeST_BoneTrackingData UpdatedSmearEndLocations true UpdatedPreviousLocations CatchupSpeed)))