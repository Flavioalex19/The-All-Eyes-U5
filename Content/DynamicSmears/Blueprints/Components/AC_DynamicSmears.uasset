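; Actor component that drives motion smear effects on the owner's mesh through dynamic material instances.
; For skeletal meshes, each bone smear gets a runtime updater component, drawn every tick into a shared float render target the materials read.
; A spawned, attached manager actor owns those components so they can be destroyed.
; Other meshes use an interpolated trailing actor vector; switching off waits on an estimated catch-up time.
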(event Custom|Update%20Smears
  ;[1 1 1] Main material update loop
  (Utilities|FlowControl|Sequence
    (:then_0
      (Variables|SkinnedMeshHandling|GetSkinnedMesh
        (:then
          (CallFunction|UpdateRuntimeComponents))
        (:else
          (if (Variables|Default|GetPerformUpdates)
            (CallFunction|UpdateActorSmearVector (Math|Float|SelectFloat (Variables|Settings|GetSmearCatchUpSpeed) (Variables|Settings|GetSmearCatchUpSpeedWhenOff) (Variables|Default|GetEnabled)))))))
    (:then_1
      (Utilities|FlowControl|DelayUntilNextTick)
      (CallFunction|UpdateSmears) ; Call itself every tick
    )))

(event Custom|Toggle
  (params (Enabled :type Boolean))
  ;[1 1 1] Toggle behavior
  (Utilities|FlowControl|Sequence
    (:then_0
      (if (and (not (Variables|Default|GetEnabled)) Enabled)
        (Variables|SkinnedMeshHandling|GetSkinnedMesh
          (:then
            (CallFunction|StartBoneSmears (Utilities|Struct|MakeST_BoneSmearData (Variables|Settings|GetTrackedBones) (Variables|Settings|GetNegatingBones) (Variables|Settings|GetDefaultDensity) (Variables|Settings|GetPullAngle) (Variables|Settings|GetMidpoint) (Variables|Settings|GetSpikeVariation) (Variables|Settings|GetMaxDistanceFromBone) (Variables|Settings|GetSmearCatchUpSpeed) (Variables|Settings|GetSmearCatchUpSpeedWhenOff) (Variables|Settings|GetBone%20to%20Smear%20Max%20Angle) (Variables|Settings|GetSmearAngleCatchupSpeed))))
          (:else))))
    (:then_1
      (Variables|Default|SetEnabled Enabled))
    (:then_2
      (if Enabled
        (Variables|Default|SetPerformUpdates true)
        (else
          (CallFunction|StopBoneSmears))))
    (:then_3
      (bind _keys (Utilities|Map|Keys (Variables|Default|GetSharedBoneTrackingData)))
      ;;[1 1 1] Add delay on deactivation to give smear time to catch up before getting turned off
      (Utilities|FlowControl|RetriggerableDelay (Math|Float|SelectFloat 0.0 (/ (CallFunction|GetSmearTimeLefttoTarget _keys -1.0) (Class|GameplayStatics|GetGlobalTimeDilation)) Enabled))
      (Utilities|FlowControl|Sequence
        (:then_0
          (for _array_element (Variables|Default|GetMaterialInstances)
            (Rendering|Material|SetScalarParameterValue _array_element "Enabled" (Math|Float|SelectFloat 1.0 0.0 Enabled) :!class /Script/Engine.MaterialInstanceDynamic)))
        (:then_1
          (Variables|Default|SetPerformUpdates Enabled))))))

(event EventBeginPlay
  (Variables|SkinnedMeshHandling|SetSkinnedMesh (Actor|GetComponentbyClass (Components|GetOwner) "/Script/Engine.SkeletalMeshComponent"))
  (Utilities|FlowControl|Sequence
    (:then_0
      (Variables|SkinnedMeshHandling|GetSkinnedMesh
        (:then
          (CallFunction|CreateRuntimeComponentsManager)
          (CallFunction|CreateRenderTarget)
          (CallFunction|IssueWarningsifNeeded))
        (:else)))
    (:then_1
      (CallFunction|InitializeVariables)
      (CallFunction|Toggle (Variables|Settings|GetStartEnabled))
      ;[1 1 1] Start ticking logic
      (CallFunction|UpdateSmears))))

(fn IssueWarningsifNeeded
  (bind _pointsperbone (Variables|Settings|GetPointsPerBone))
  (bind _values (Utilities|Map|Values _pointsperbone))
  (for _array_element _values
    (LocalVariables|SettotalPointsRequired (+ _array_element (LocalVariables|GettotalPointsRequired))))
  (for _index (range 1 (- (+ (Utilities|Array|Length (Variables|Settings|GetTrackedBones)) (Utilities|Array|Length (Variables|Settings|GetNegatingBones))) (Utilities|Map|Length _pointsperbone)))
    (LocalVariables|SettotalPointsRequired (+ (Variables|Settings|GetPointsPerBoneDefault) (LocalVariables|GettotalPointsRequired))))
  (if (> (LocalVariables|GettotalPointsRequired) (Variables|SkinnedMeshHandling|GetTotalPointsSupported))
    (Development|PrintString (Utilities|String|Append "DYNAMIC SMEARS: YOUR SETTINGS REQUIRES SUPPORTING " (Utilities|String|ToString(Integer) (LocalVariables|GettotalPointsRequired)) " POINTS, BUT YOUR SMEAR RENDER TARGET ONLY SUPPORTS UP TO " (Utilities|String|ToString(Integer) (Variables|SkinnedMeshHandling|GetTotalPointsSupported)) "!") true true "(R=1.000000,G=0.000000,B=0.074582,A=1.000000)" 6e+01)))

(fn InitializeVariables
  (bind _returnvalue (Components|GetOwner))
  (bind _returnvalue_2 (Actor|GetComponentbyClass _returnvalue "/Script/Engine.MeshComponent"))
  (Utilities|FlowControl|Sequence
    (:then_0
      ;[1 1 1] Convert materials to dynamic material instances
      (for (_array_element _array_index) (Rendering|Material|GetMaterials _returnvalue_2)
        (Utilities|IsValid _array_element
          (:Is%20Valid
            (bind _returnvalue_3 (Rendering|Material|CreateDynamicMaterialInstance _array_element "None" "None" :!class /Script/Engine.KismetMaterialLibrary))
            (Rendering|Material|SetMaterial _returnvalue_2 _array_index _returnvalue_3)
            (Utilities|Array|Add (Variables|Default|GetMaterialInstances) _returnvalue_3)))))
    (:then_1
      (CallFunction|SetSmearScalarValue "IsSkinnedMesh" (Math|Float|SelectFloat 1.0 0.0 (Utilities|IsValid (Variables|SkinnedMeshHandling|GetSkinnedMesh))))
      (CallFunction|SetSmearTextureValue "RenderTargetTexture" (Variables|SkinnedMeshHandling|GetSmearRenderTarget))
      ;[1 1 1] Only used if not a skinned mesh
      (CallFunction|SetSmearScalarValue "Density" (Variables|Settings|GetDefaultDensity))
      (CallFunction|SetSmearScalarValue "Pull angle" (Variables|Settings|GetPullAngle))
      (CallFunction|SetSmearScalarValue "Spike variation" (Variables|Settings|GetSpikeVariation))
      (CallFunction|SetSmearScalarValue "Midpoint" (Variables|Settings|GetMidpoint))
      (CallFunction|SetSmearScalarValue "MaxDistanceFromBone" (Variables|Settings|GetMaxDistanceFromBone)))))

(fn SaveTrackedBoneData
  (params (TrackedBones :type Array%20of%20Names) (NegatingBones :type Array%20of%20Names))
  (LocalVariables|SetSocketAndBoneNames (Transformation|GetAllSocketNames (Variables|SkinnedMeshHandling|GetSkinnedMesh)))
  (Utilities|Array|AppendArray (LocalVariables|GetBonesToRecord) TrackedBones)
  (Utilities|Array|AppendArray (LocalVariables|GetBonesToRecord) NegatingBones)
  (for _array_element (LocalVariables|GetBonesToRecord)
    (if (>= (Class|SkinnedMeshComponent|GetBoneIndex (Variables|SkinnedMeshHandling|GetSkinnedMesh) _array_element) 0)
      _
      (else
        (Development|PrintString (Utilities|String|Append "DYNAMIC SMEARS: THERE IS NO BONE CALLED " (Utilities|String|ToString(Name) _array_element) "!! YOU WILL GET STRANGE RESULT IF YOU DON'T USE AN EXISTING BONE'S NAME") true true "(R=1.000000,G=0.019646,B=0.000000,A=1.000000)" 6e+01)))
    (LocalVariables|SetCurrentBoneIndex (Class|SkinnedMeshComponent|GetBoneIndex (Variables|SkinnedMeshHandling|GetSkinnedMesh) _array_element))
    (LocalVariables|SetCurrentBoneTransform (Transformation|GetBoneTransform (Variables|SkinnedMeshHandling|GetSkinnedMesh) _array_element "RTS_World"))
    (for _array_element_2 (LocalVariables|GetSocketAndBoneNames)
      (if (== (Class|SkinnedMeshComponent|GetBoneIndex (Variables|SkinnedMeshHandling|GetSkinnedMesh) _array_element_2) (+ (LocalVariables|GetCurrentBoneIndex) 1))
        ;[1 1 1] Record length if there is no record yet, or if the found length is longer than the recorded one
        (if (.ReturnValue (Utilities|Map|Find (Variables|SkinnedMeshHandling|GetBoneLengths) _array_element))
          (if (> (Math|Vector|VectorLength (- (.location (Transformation|GetBoneTransform (Variables|SkinnedMeshHandling|GetSkinnedMesh) _array_element_2 "RTS_World")) (.location (LocalVariables|GetCurrentBoneTransform)))) (.Value (Utilities|Map|Find (Variables|SkinnedMeshHandling|GetBoneLengths) _array_element)))
            (Utilities|Map|Add (Variables|SkinnedMeshHandling|GetBoneLengths) _array_element (Math|Vector|VectorLength (- (.location (Transformation|GetBoneTransform (Variables|SkinnedMeshHandling|GetSkinnedMesh) _array_element_2 "RTS_World")) (.location (LocalVariables|GetCurrentBoneTransform)))) :!label _label)
            (Utilities|Map|Add (Variables|SkinnedMeshHandling|GetBoneChildName) _array_element _array_element_2))
          (else
            (goto _label)))))
    ;[1 1 1] If the bone has no child, set is length to a default of 0
    (if (not (.ReturnValue (Utilities|Map|Find (Variables|SkinnedMeshHandling|GetBoneLengths) _array_element)))
      (Utilities|Map|Add (Variables|SkinnedMeshHandling|GetBoneLengths) _array_element 0.0))))

(fn UpdateActorSmearVector
  (params (SmearCatchUpSpeedToUse :type Float%20%28single-precision%29))
  (for _array_element (Variables|Default|GetMaterialInstances)
    (Rendering|Material|SetVectorParameterValue _array_element "VectorToPrevious" (Math|Conversions|ToLinearColor(Vector) (- (Variables|Default|GetSmearEndLocation) (Transformation|GetActorLocation (Components|GetOwner)))) :!class /Script/Engine.MaterialInstanceDynamic))
  (Variables|Default|SetSmearEndLocation (Math|Interpolation|VInterpTo (Variables|Default|GetSmearEndLocation) (Transformation|GetActorLocation (Components|GetOwner)) (Utilities|Time|GetWorldDeltaSeconds) SmearCatchUpSpeedToUse)))

(fn SetSmearScalarValue
  (params (ParameterName :type Name) (Value :type Float%20%28single-precision%29))
  (for _array_element (Variables|Default|GetMaterialInstances)
    (Rendering|Material|SetScalarParameterValue _array_element ParameterName Value :!class /Script/Engine.MaterialInstanceDynamic)))

(fn SetSmearTextureValue
  (params (ParameterName :type Name) (Value :type Texture%20Object%20Reference))
  (for _array_element (Variables|Default|GetMaterialInstances)
    (Rendering|Material|SetTextureParameterValue _array_element ParameterName Value)))

(fn SaveDatatoRenderTarget
  (params (Canvas :type Canvas%20Object%20Reference) (Pixel%20X :type Integer) (Pixel%20Y :type Integer) (Data :type Linear%20Color%20Structure))
  (Canvas|DrawTexture :self Canvas :ScreenPosition (Math|Vector2D|MakeVector2D (Math|Conversions|ToFloat(Integer) Pixel%20X) (Math|Conversions|ToFloat(Integer) Pixel%20Y)) :ScreenSize "(X=1.000000,Y=1.000000)" :CoordinateSize "(X=1.000000,Y=1.000000)" :RenderColor Data :BlendMode "BLEND_Opaque" :PivotPoint "(X=0.000000,Y=0.000000)"))

(fn CreateRenderTarget
  (bind _returnvalue (Rendering|CreateRenderTarget2D 1024 16 "RTF_RGBA32f" "(R=0.000000,G=0.000000,B=0.000000,A=1.000000)" false true))
  (bind _output_get (Variables|SkinnedMeshHandling|SetSmearRenderTarget _returnvalue))
  (Variables|/Script/Engine.Texture|SetLODGroup _output_get "TEXTUREGROUP_Pixels2D")
  (Variables|/Script/Engine.TextureRenderTarget2D|SetAddressX _output_get "TA_Clamp")
  (Variables|/Script/Engine.TextureRenderTarget2D|SetAddressY _output_get "TA_Clamp")
  (Variables|SkinnedMeshHandling|SetTotalPointsSupported (Variables|/Script/Engine.TextureRenderTarget2D|GetSizeX _output_get)))

(fn UpdateRuntimeComponents
  (if (Utilities|Array|IsNotEmpty (Variables|Default|GetSmearsToUpdate))
    (Rendering|ClearRenderTarget2D (Variables|SkinnedMeshHandling|GetSmearRenderTarget))
    (CallFunction|MarkSharedBoneDataasPendingUpdate)
    (bind (_canvas _size _context) (Rendering|BeginDrawCanvastoRenderTarget (Variables|SkinnedMeshHandling|GetSmearRenderTarget)))
    (Variables|Default|SetRTColIndex 0)
    (bind (_arrayindex _arrayelement) (Utilities|Array|ReverseforEachLoop (Variables|Default|GetSmearsToUpdate))
      (:LoopBody
        (bind _output_get (LocalVariables|SetComponent _arrayelement))
        (if (Variables|/Game/DynamicSmears/Blueprints/Components/RAC_RUNTIME_COMPONENT_SmearUpdater.RAC_RUNTIME_COMPONENT_SmearUpdater_C|GetEnabled _output_get)
          (Default|Update (LocalVariables|GetComponent) _canvas)
          (else
            (Utilities|Array|RemoveIndex (Variables|Default|GetSmearsToUpdate) _arrayindex)
            ;[1 1 1] Remove unnecessary tracking data and delete component
            (for _array_element (.TrackedBones (Utilities|Struct|BreakST_BoneSmearData (Variables|/Game/DynamicSmears/Blueprints/Components/RAC_RUNTIME_COMPONENT_SmearUpdater.RAC_RUNTIME_COMPONENT_SmearUpdater_C|GetSmearData (LocalVariables|GetComponent))))
              (if (not (CallFunction|IsBoneStillTracked _array_element))
                (Utilities|Map|Remove (Variables|Default|GetSharedBoneTrackingData) _array_element)))
            (Default|DestroyLocalComponent (Variables|Default|GetRuntimeComponentsManager) (LocalVariables|GetComponent)))))
      (:Completed
        (Rendering|EndDrawCanvastoRenderTarget _context)))))

(fn StartBoneSmears
  (params (SmearData :type ST%20Bone%20Smear%20Data%20Structure) (OwningANS :type Anim%20Notify%20State%20Object%20Reference%20%28by%20ref%29))
  (bind (_trackedbones _negatingbones) (Utilities|Struct|BreakST_BoneSmearData SmearData))
  (CallFunction|SaveTrackedBoneData _trackedbones _negatingbones)
  (CallFunction|SetSmearScalarValue "Enabled" 1.0)
  (bind _returnvalue (Game|AddComponentbyClass (Variables|Default|GetRuntimeComponentsManager) "/Game/DynamicSmears/Blueprints/Components/RAC_RUNTIME_COMPONENT_SmearUpdater.RAC_RUNTIME_COMPONENT_SmearUpdater_C"))
  (bind _smear (Default|Initialize _returnvalue self OwningANS (Variables|Default|GetMaterialInstances) (Variables|SkinnedMeshHandling|GetSkinnedMesh) (Variables|SkinnedMeshHandling|GetSmearRenderTarget) SmearData (Variables|Settings|GetPointsPerBone) (Variables|SkinnedMeshHandling|GetBoneLengths) (Variables|SkinnedMeshHandling|GetBoneChildName)))
  (Utilities|Array|Add (Variables|Default|GetSmearsToUpdate) _smear)
  (return _smear))

(fn StopBoneSmears
  (params (Owning%20ANS :type Anim%20Notify%20State%20Object%20Reference%20%28by%20ref%29))
  (bind _array_element (Utilities|Array|ForEachLoopwithBreak (Variables|Default|GetSmearsToUpdate) :!label _label)
    (:LoopBody
      (if (== (Variables|/Game/DynamicSmears/Blueprints/Components/RAC_RUNTIME_COMPONENT_SmearUpdater.RAC_RUNTIME_COMPONENT_SmearUpdater_C|GetOwning%20ANS _array_element) Owning%20ANS)
        (Default|FadeOff _array_element)
        (goto _label Break)))
    (:Completed
      (if (Utilities|Array|IsEmpty (Variables|Default|GetSmearsToUpdate))
        (CallFunction|SetSmearScalarValue "Enabled" 0.0)))))

(fn CreateRuntimeComponentsManager
  ;[1 1 1] We need to spawn an actor to hold and destroy the components we will create at runtime, as you can only destroy components from the actor who created them. This allow the dynamic smears logic to work without having to modify the actor it is attached to to handle that logic.
  (bind _returnvalue (Game|SpawnActorfromClass "/Game/DynamicSmears/Blueprints/BP_DynamicSmearsRuntimeComponentManager.BP_DynamicSmearsRuntimeComponentManager_C" (Math|Transform|MakeTransform "0, 0, 0") "DontSpawnIfColliding" "MultiplyWithRoot" (Components|GetOwner) 0))
  (bind _output_get (Variables|Default|SetRuntimeComponentsManager _returnvalue))
  (Transformation|AttachActorToActor _output_get (Components|GetOwner) "None" "SnapToTarget" "SnapToTarget" "SnapToTarget" true))

(fn MarkSharedBoneDataasPendingUpdate
  (bind _sharedbonetrackingdata (Variables|Default|GetSharedBoneTrackingData))
  (bind _keys (Utilities|Map|Keys (Variables|Default|GetSharedBoneTrackingData)))
  (for _array_element _keys
    (Utilities|Map|Add _sharedbonetrackingdata _array_element (Utilities|Struct|MakeST_BoneTrackingData (.SmearEndLocations (Utilities|Struct|BreakST_BoneTrackingData (.Value (Utilities|Map|Find _sharedbonetrackingdata _array_element)))) false (.PreviousLocations (Utilities|Struct|BreakST_BoneTrackingData (.Value (Utilities|Map|Find _sharedbonetrackingdata _array_element)))) 0.0))))

(fn IsBoneStillTracked
  (params (Bone :type Name))
  (for _array_element (Variables|Default|GetSmearsToUpdate)
    (if (Utilities|Array|ContainsItem (.TrackedBones (Utilities|Struct|BreakST_BoneSmearData (Variables|/Game/DynamicSmears/Blueprints/Components/RAC_RUNTIME_COMPONENT_SmearUpdater.RAC_RUNTIME_COMPONENT_SmearUpdater_C|GetSmearData _array_element))) Bone)
      (return true)))
  (return false))

(fn GetSmearTimeLefttoTarget
  (params (BonesToConsider :type Array%20of%20Names) (OverrideCatchupSpeed :type Float%20%28double-precision%29))
  (for _array_element BonesToConsider
    (if (.ReturnValue (Utilities|Map|Find (Variables|Default|GetSharedBoneTrackingData) _array_element))
      (for (_array_element_2 _array_index) (.SmearEndLocations (Utilities|Struct|BreakST_BoneTrackingData (.Value (Utilities|Map|Find (Variables|Default|GetSharedBoneTrackingData) _array_element))))
        (if (or (> (/ (Math|Float|Log (Math|Vector|Distance(Vector) _array_element_2 (Utilities|Array|Get(acopy) (.PreviousLocations (Utilities|Struct|BreakST_BoneTrackingData (.Value (Utilities|Map|Find (Variables|Default|GetSharedBoneTrackingData) _array_element)))) _array_index)) 2.0) (Math|Float|SelectFloat OverrideCatchupSpeed (.OffCatchupSpeed (Utilities|Struct|BreakST_BoneTrackingData (.Value (Utilities|Map|Find (Variables|Default|GetSharedBoneTrackingData) _array_element)))) (> OverrideCatchupSpeed 0.0))) (LocalVariables|GetLongestTimeLeft)) (< (LocalVariables|GetLongestTimeLeft) 0.0))
          (LocalVariables|SetLongestTimeLeft (/ (Math|Float|Log (Math|Vector|Distance(Vector) _array_element_2 (Utilities|Array|Get(acopy) (.PreviousLocations (Utilities|Struct|BreakST_BoneTrackingData (.Value (Utilities|Map|Find (Variables|Default|GetSharedBoneTrackingData) _array_element)))) _array_index)) 2.0) (Math|Float|SelectFloat OverrideCatchupSpeed (.OffCatchupSpeed (Utilities|Struct|BreakST_BoneTrackingData (.Value (Utilities|Map|Find (Variables|Default|GetSharedBoneTrackingData) _array_element)))) (> OverrideCatchupSpeed 0.0))))))))
  (return (Math|Float|SelectFloat (LocalVariables|GetLongestTimeLeft) 0.0 (> (LocalVariables|GetLongestTimeLeft) 0.0))))